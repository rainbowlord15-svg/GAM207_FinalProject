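; Player character Blueprint that moves, looks around and fires projectiles.
; Enhanced Input actions feed movement along the actor's forward and right vectors, and look input turns the controller with inverted pitch.
; Left mouse press spawns BP_Projectile at the Projectilespawnlocation component's transform, always spawning regardless of collisions, through a raw key event rather than an input action.
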(event `Key|LeftMouseButton`
  (params (Key :type "Key Structure"))
  (:`Pressed`
    (`|SpawnActorFromClass` "/Game/BP_Projectile.BP_Projectile_C" (`SceneComponent.K2_GetComponentToWorld` (`self.projectilespawnlocation`)) "AlwaysSpawn" "MultiplyWithRoot" null null)))

(event `EnhancedInput|/Game/IA_Movement`
  (params (ActionValue :type "Vector2D Structure") (ElapsedSeconds :type "Float (double-precision)") (TriggeredSeconds :type "Float (double-precision)") (InputAction :type "InputAction Object Reference" :default "/Game/IA_Movement.IA_Movement"))
  (bind (_x _y) (`KismetMathLibrary.BreakVector2D` ActionValue))
  (:`Triggered`
    (`self.AddMovementInput` (`self.GetActorForwardVector`) _y)
    (`self.AddMovementInput` (`self.GetActorRightVector`) _x)))

(event `EnhancedInput|/Game/IA_Look`
  (params (ActionValue :type "Vector2D Structure") (ElapsedSeconds :type "Float (double-precision)") (TriggeredSeconds :type "Float (double-precision)") (InputAction :type "InputAction Object Reference" :default "/Game/IA_Look.IA_Look"))
  (bind (_x _y) (`KismetMathLibrary.BreakVector2D` ActionValue))
  (:`Triggered`
    (`self.AddControllerYawInput` _x)
    (`self.AddControllerPitchInput` (* _y -1.0))))

(fn `UserConstructionScript`)